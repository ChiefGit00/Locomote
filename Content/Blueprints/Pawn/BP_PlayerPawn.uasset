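; Touch-controlled player pawn for a tile-based level, with a sphere that moves between tiles and a spring-arm camera.
; MoveToTile drives a timeline that lerps the sphere toward the target location.
; A gated Tick, open while Finger1 is down, turns swipes past a threshold into camera yaw, or spring-arm panning with two fingers.
; After a short delay, BeginPlay registers the overlapped starting tile with BP_PlayerCtrl_Levels and marks it walked.
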(event `MoveToTile`
  (params (NewLocation :type "Vector Structure"))
  (bind _sphere (`self.Sphere`))
  ;[1 1 1 1 40] MoveToTile
  (bind (_direction _float) (`Timeline|Timeline_MoveTo` :!via `PlayFromStart`)
    (:`Update`
      (`SceneComponent.K2_SetWorldLocation` _sphere (`KismetMathLibrary.VLerp` (`SceneComponent.K2_GetComponentLocation` _sphere) NewLocation _float) false false))))

(event `self.ReceiveTick`
  (params (DeltaSeconds :type "Float (single-precision)"))
  (bind _springarm (`self.SpringArm`))
  (bind (_locationx _locationy _biscurrentlypressed) (`PlayerController.GetInputTouchState` (`GameplayStatics.GetPlayerController` 0) "Touch1"))
  (bind _returnvalue (`KismetMathLibrary.MakeVector2D` _locationx _locationy))
  (bind _returnvalue_2 (- _returnvalue (`self.EndLoc`)))
  (bind (_returnvalue_x _returnvalue_y) (`KismetMathLibrary.BreakVector2D` (* _returnvalue_2 (`self.SwipeSpeed`))))
  (bind (_x _y) (`KismetMathLibrary.BreakVector2D` _returnvalue_2))
  ;[0.07292 0.07292 0.07292 0.2 40] Camera Rotate and Zoom
  (`/Engine/EditorBlueprintResources/StandardMacros.Gate` true :!label _label
    (:`Exit`
      (if (>= (`KismetMathLibrary.VSize2D` (- _returnvalue (stale `InputAction|Finger1` _output_get))) (`self.SwipeThreshold`))
        (set `self.StartLoc` (100000.0 100000.0))
        (if (and _biscurrentlypressed (`.bIsCurrentlyPressed` (`PlayerController.GetInputTouchState` (`GameplayStatics.GetPlayerController` 0) "Touch2")))
          (`SceneComponent.K2_AddRelativeLocation` _springarm (`KismetMathLibrary.MakeVector` _y (- 0.0 _x)) false false)
          (else
            (`SceneComponent.K2_AddRelativeRotation` _springarm (`KismetMathLibrary.MakeRotator` 0.0 0.0 _returnvalue_x) false false)))
        (set `self.EndLoc` _returnvalue)))))

(event `InputAction|Finger1`
  (params (Key :type "Key Structure"))
  (bind (_locationx _locationy _biscurrentlypressed) (`PlayerController.GetInputTouchState` (`GameplayStatics.GetPlayerController` 0) "Touch1"))
  ;[0.07292 0.07292 0.07292 0.2 40] Camera Rotate and Zoom
  (:`Pressed`
    (bind _output_get (set `self.StartLoc` (`KismetMathLibrary.MakeVector2D` _locationx _locationy)))
    (set `self.EndLoc` _output_get)
    (goto _label :!via `Open`))
  (:`Released`
    (goto _label :!via `Close`)))

(event `self.ReceiveBeginPlay`
  ;[1 1 1 1 40] Begin Play
  (`KismetSystemLibrary.Delay` 0.2)
  (bind _asbp_tile_base (cast `/Game/Blueprints/Actors/BP_Tile_base` (`|GetArrayItem` (`PrimitiveComponent.GetOverlappingActors` (`self.Sphere1`) "/Game/Blueprints/Actors/BP_Tile_base.BP_Tile_Base_C"))))
  (bind _output_get (set `/Game/Blueprints/Game/BP_PlayerCtrl_Levels.LastTile` _asbp_tile_base (`self.PlayerCtrl`)))
  (`/Game/Blueprints/Actors/BP_Tile_base.OnWalked` _output_get))

(event `self.ReceivePossessed`
  (params (NewController :type "Controller Object Reference"))
  (bind _asbp_player_ctrl_levels (cast `/Game/Blueprints/Game/BP_PlayerCtrl_Levels` NewController))
  (set `self.PlayerCtrl` _asbp_player_ctrl_levels))

(fn `ResetLocation`
  (`self.K2_SetActorTransform` (`KismetMathLibrary.MakeTransform` (0.0 0.0 27.0))))

(fn `UserConstructionScript`)