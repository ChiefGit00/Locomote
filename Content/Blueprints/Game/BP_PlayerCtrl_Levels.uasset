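; Player controller for tile-based levels, running a turn-limited move loop with win and out-of-turns outcomes.
; Set starts a round by setting turns, rebuilding the HUD, resetting the pawn and fetching its start tile.
; Move, blocked while swiping, spends a turn, updates tiles and moves the pawn.
; A goal tile saves XP through the game instance and shows the win screen; exhausted turns show the failure screen, both pausing the game.
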(event `self.ReceiveBeginPlay`)

(event `self.ReceivePossess`
  (params (PossessedPawn :type "Pawn Object Reference"))
  (bind _asbp_player_pawn (cast `/Game/Blueprints/Pawn/BP_PlayerPawn` PossessedPawn))
  (set `self.PlayerPawn` _asbp_player_pawn))

(event `TurnsFinish`
  (`KismetSystemLibrary.Delay` 0.7)
  (`Widget.RemoveFromParent` (`self.UI_HUD`))
  (`GameplayStatics.SetGamePaused` true)
  (bind _returnvalue (`|CreateWidget` "/Game/UI/UI_TurnsFinish.UI_TurnsFinish_C"))
  (`UserWidget.AddToViewport` _returnvalue 0))

(event `Win`
  (bind _xp (`/Game/Blueprints/Actors/Tiles/BP_Tile_Base.GetXPAward` (`self.LastTile`)))
  (bind _asbp_game_instance (cast `/Game/Blueprints/Game/BP_GameInstance` (`GameplayStatics.GetGameInstance`)))
  (bind (_firstxp _earnedxp _totalxp _key) (`/Game/Blueprints/Game/BP_GameInstance.SaveCurrentXP` _asbp_game_instance _xp))
  (`KismetSystemLibrary.Delay` 0.7)
  (`GameplayStatics.SetGamePaused` true)
  (`WidgetLayoutLibrary.RemoveAllWidgets`)
  (bind _returnvalue (`|CreateWidget` "/Game/UI/UI_Win.UI_Win_C"))
  (`/Game/UI/UI_Win.XPEarnerd` _returnvalue _firstxp _earnedxp _totalxp _key)
  (`UserWidget.AddToViewport` _returnvalue 0))

(event `Set`
  (params (Turns :type Integer))
  (bind _playerpawn (`self.PlayerPawn`))
  (set `self.Turns` Turns)
  (`GameplayStatics.SetGamePaused` false)
  (`WidgetLayoutLibrary.RemoveAllWidgets`)
  (`self.HUD`)
  (`/Game/Blueprints/Pawn/BP_PlayerPawn.Reset` _playerpawn)
  (`KismetSystemLibrary.Delay` 0.5)
  (`/Game/Blueprints/Pawn/BP_PlayerPawn.GetStartTile` _playerpawn))

(fn `Move`
  (params (NewLocation :type "Vector Structure") (TileTo :type "/Game/Blueprints/Actors/Tiles/BP_Tile_Base Object Reference"))
  (bind _lasttile (`self.LastTile`))
  (if (`self.bSwipe`)
    _
    (elif (> (`self.Turns`) 0)
      (`/Engine/EditorBlueprintResources/StandardMacros.DecrementInt` (`self.Turns`)
        (:`  `
          (`/Game/Blueprints/Actors/Tiles/BP_Tile_Base.DeactivateUnused` _lasttile (`/Game/Blueprints/Actors/Tiles/BP_Tile_Base.NeighbourActivationCount` _lasttile) false)
          (bind _output_get (set `self.LastTile` TileTo))
          (`/Game/Blueprints/Actors/Tiles/BP_Tile_Base.OnWalked` _output_get)
          (`/Game/Blueprints/Pawn/BP_PlayerPawn.MoveToTile` (`self.PlayerPawn`) NewLocation)
          (if (`|EnumEquality` (`/Game/Blueprints/Actors/Tiles/BP_Tile_Base.TileType` _output_get) "NewEnumerator3")
            (`self.Win`)
            (elif (== (`self.Turns`) 0)
              (`self.TurnsFinish`))))))))

(fn `UserConstructionScript`)