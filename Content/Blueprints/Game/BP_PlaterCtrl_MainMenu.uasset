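; Player controller for the main menu that switches between the menu and settings screens.
; On BeginPlay it calls its MainMenu event to show the UI_MainMenu_temp widget.
; MainMenu and a separate Settings event each clear all widgets, create a fresh screen widget, add it to the viewport and show the mouse cursor.
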(event `self.ReceiveBeginPlay`
  (`self.MainMenu`))

(event `MainMenu`
  (`WidgetLayoutLibrary.RemoveAllWidgets`)
  (bind _returnvalue (`|CreateWidget` "/Game/UI/UI_MainMenu_temp.UI_MainMenu_temp_C"))
  (`UserWidget.AddToViewport` _returnvalue 0)
  (set `self.bShowMouseCursor` true))

(event `Settings`
  (`WidgetLayoutLibrary.RemoveAllWidgets`)
  (bind _returnvalue (`|CreateWidget` "/Game/UI/UI_Settings.UI_Settings_C"))
  (`UserWidget.AddToViewport` _returnvalue 0)
  (set `self.bShowMouseCursor` true))

(fn `UserConstructionScript`)