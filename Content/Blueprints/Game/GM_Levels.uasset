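; GM_Levels is the game mode that handles level selection and spawns levels as actors.
; On BeginPlay it calls OpenLevelByName with the current level stored in BP_GameInstance.
; OpenLevel only accepts unlocked levels, records the current one, and spawns the level Blueprint listed in DT_Levels.
; It then resets the player pawn's location and copies the spawned level's starting turn count to the player controller.
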(event `self.ReceiveBeginPlay`
  (bind _asbp_game_instance (cast `/Game/Blueprints/Game/BP_GameInstance` (`GameplayStatics.GetGameInstance`)))
  (`self.OpenLevel` (`/Game/Blueprints/Game/BP_GameInstance.CurrentLevel` _asbp_game_instance)))

(fn `OpenLevel`
  (params (Level :type Integer))
  (if (<= Level (`self.UnlockedLevel`))
    (set `self.CurrentLevel` Level)
    (bind _returnvalue (`|GetDataTableRow` "/Game/Data/DT_Levels.DT_Levels" (`KismetStringLibrary.Conv_StringToName` (`KismetStringLibrary.Conv_IntToString` Level)))
      (:`then`
        (bind _returnvalue_2 (`|SpawnActorFromClass` (`.BP_Level_5_0017295045148736FF82D683BCDB3EE1` (break `/Game/Data/F_Levels` _returnvalue)) (`KismetMathLibrary.MakeTransform` (0.0 0.0 0.0)) "Undefined" "OverrideRootScale" null null))
        (bind _asbp_player_pawn (cast `/Game/Blueprints/Pawn/BP_PlayerPawn` (`GameplayStatics.GetPlayerPawn` 0)))
        (`/Game/Blueprints/Pawn/BP_PlayerPawn.ResetLocation` _asbp_player_pawn)
        (bind _asbp_player_ctrl_levels (cast `/Game/Blueprints/Game/BP_PlayerCtrl_Levels` (`GameplayStatics.GetPlayerController` 0)))
        (set `/Game/Blueprints/Game/BP_PlayerCtrl_Levels.Turns` (`/Game/Blueprints/Actors/BP_Level.StartTurns` _returnvalue_2) _asbp_player_ctrl_levels)))))

(fn `UserConstructionScript`)