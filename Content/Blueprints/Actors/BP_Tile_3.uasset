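; BP_Tile_3 is a child tile actor for a walkable tile puzzle, with a top-face widget that shows its neighbour activation count.
; On BeginPlay it rebuilds its box collider list from X, Y and diagonal colliders, several repeated, then calls GetNeighbours.
; SetTileType runs the parent logic, then shows the count only on Can Walk tiles and hides the widget for all other states.
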(event `self.ReceiveBeginPlay`
  (bind _boxcolls (`self.BoxColls`))
  (`KismetArrayLibrary.Array_Clear` _boxcolls)
  (`KismetArrayLibrary.Array_Add` _boxcolls (`self.Coll_X+`))
  (`KismetArrayLibrary.Array_Add` _boxcolls (`self.Coll_X-`))
  (`KismetArrayLibrary.Array_Add` _boxcolls (`self.Coll_Y+`))
  (`KismetArrayLibrary.Array_Add` _boxcolls (`self.Coll_Y-`))
  (`KismetArrayLibrary.Array_Add` _boxcolls (`self.Coll_X+Y+`))
  (`KismetArrayLibrary.Array_Add` _boxcolls (`self.Coll_X-Y+`))
  (`KismetArrayLibrary.Array_Add` _boxcolls (`self.Coll_X-Y-`))
  (`KismetArrayLibrary.Array_Add` _boxcolls (`self.Coll_Y-X+`))
  (`self.GetNeighbours`))

(fn `SetTileType`
  (params (TileType :type "/Game/Data/E_TileType Enum" :default "NewEnumerator0"))
  (`parent.SetTileType` TileType)
  (bind _asui_tile_top (cast `/Game/UI/UI_TileTop` (`WidgetComponent.GetUserWidgetObject` (`self.Widget`))))
  (switch `/Game/Data/E_TileType` (`self.TileType`)
    (:`NewEnumerator0`
      (`/Game/UI/UI_TileTop.Visible` _asui_tile_top false))
    (:`NewEnumerator1`
      (`/Game/UI/UI_TileTop.SetCount` _asui_tile_top (`self.NeighbourActivationCount`))
      (`/Game/UI/UI_TileTop.Visible` _asui_tile_top true)
      (`/Game/UI/UI_TileTop.Visible` _asui_tile_top true))
    (:`NewEnumerator2`
      (`/Game/UI/UI_TileTop.Visible` _asui_tile_top false :!label _label))
    (:`NewEnumerator3`
      (goto _label))
    (:`NewEnumerator4`
      (goto _label))))

(fn `UserConstructionScript`
  (`parent.UserConstructionScript`))