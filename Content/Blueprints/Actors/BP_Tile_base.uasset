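; Base actor for a walkable puzzle tile: a click or touch moves the player pawn onto it if walkable.
; SetTileType sets the state and top material, and OnWalked marks a tile Walked, then recurses through neighbours to a set depth to unlock tiles, including Finish.
; Neighbours come from overlap queries on box colliders.
; Player overlap on a Finish tile triggers a delayed Win with the parent level's XP award.
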(event `self.StaticMesh.OnClicked`
  (params (TouchedComponent :type "PrimitiveComponent Object Reference") (ButtonPressed :type "Key Structure"))
  (`self.OnClicked/Touched` :!label _label))

(event `self.StaticMesh.OnInputTouchBegin`
  (params (FingerIndex :type "ETouchIndex Enum" :default "Touch1") (TouchedComponent :type "PrimitiveComponent Object Reference"))
  (goto _label))

(event `self.Box.OnComponentBeginOverlap`
  (params (OverlappedComponent :type "PrimitiveComponent Object Reference") (OtherActor :type "Actor Object Reference") (OtherComp :type "PrimitiveComponent Object Reference") (OtherBodyIndex :type Integer) (bFromSweep :type Boolean) (SweepResult :type "HitResult Structure (by ref)"))
  (cast `/Game/Blueprints/Pawn/BP_PlayerPawn` OtherActor)
  (switch `/Game/Data/E_TileType` (`self.TileType`)
    (:`NewEnumerator3`
      (bind _asbp_player_ctrl_levels (cast `/Game/Blueprints/Game/BP_PlayerCtrl_Levels` (`GameplayStatics.GetPlayerController` 0)))
      (bind _asbp_level (cast `/Game/Blueprints/Actors/BP_Level` (`self.GetParentActor`)))
      (`KismetSystemLibrary.Delay` 0.2)
      (`/Game/Blueprints/Game/BP_PlayerCtrl_Levels.Win` _asbp_player_ctrl_levels (`/Game/Blueprints/Actors/BP_Level.XPAward` _asbp_level)))))

(fn `ActivateNeighbours`
  (params (Count :type Integer))
  (bind _neighbourtiles (`self.NeighbourTiles`))
  (if (== Count 0)
    (for _array_element _neighbourtiles
      (`/Engine/EditorBlueprintResources/StandardMacros.IsValid` _array_element
        (:`Is Valid`
          (bind _tiletype (`/Game/Blueprints/Actors/BP_Tile_base.TileType` _array_element))
          (if (`|EnumEquality` _tiletype "NewEnumerator2")
            (`self.SetTileType` _array_element "NewEnumerator1")
            (elif (`|EnumEquality` _tiletype "NewEnumerator3")
              (set `/Game/Blueprints/Actors/BP_Tile_base.bCanWalk` true _array_element))))))
    (else
      (bind _result (`/Engine/EditorBlueprintResources/StandardMacros.DecrementInt` Count)
        (:`  `
          (for _array_element_2 _neighbourtiles
            (`self.ActivateNeighbours` _array_element_2 _result)))))))

(fn `GetNeighbour`
  (params (BoxCollision :type "PrimitiveComponent Object Reference"))
  (returns (Tile :type "/Game/Blueprints/Actors/BP_Tile_base Object Reference"))
  (bind (_outactors _returnvalue) (`KismetSystemLibrary.ComponentOverlapActors` BoxCollision (`SceneComponent.K2_GetComponentToWorld` BoxCollision) (`|MakeArray` "ObjectTypeQuery2" :!type "EObjectTypeQuery Enum") "/Game/Blueprints/Actors/BP_Tile.BP_Tile_C" (`|MakeArray` self :!type "Actor Object Reference")))
  (if _returnvalue
    (bind _asbp_tile_base (cast `/Game/Blueprints/Actors/BP_Tile_base` (`|GetArrayItem` _outactors)))
    (return _asbp_tile_base)
    (else
      (return null))))

(fn `GetNeighbours`
  (`KismetArrayLibrary.Array_Clear` (`self.NeighbourTiles`))
  (for _array_element (`self.BoxColls`)
    (bind _tile (`self.GetNeighbour` _array_element))
    (`/Engine/EditorBlueprintResources/StandardMacros.IsValid` _tile
      (:`Is Valid`
        (`KismetArrayLibrary.Array_Add` (`self.NeighbourTiles`) _tile)))))

(fn `OnClicked/Touched`
  (if (`self.bCanWalk`)
    (bind _asbp_player_pawn (cast `/Game/Blueprints/Pawn/BP_PlayerPawn` (`GameplayStatics.GetPlayerPawn` 0)))
    (`/Game/Blueprints/Pawn/BP_PlayerPawn.MoveToTile` _asbp_player_pawn (+ (`self.K2_GetActorLocation`) (0.0 0.0 27.0)) self)))

(fn `OnWalked`
  (if (`|EnumEquality` (`self.TileType`) "NewEnumerator1")
    (`self.SetTileType` "NewEnumerator0")
    (`self.ActivateNeighbours` (`self.NeighbourActivationCount`))))

(fn `SetTileType`
  (params (TileType :type "/Game/Data/E_TileType Enum" :default "NewEnumerator0"))
  (bind _staticmesh (`self.StaticMesh`))
  (switch `/Game/Data/E_TileType` TileType
    (:`NewEnumerator0`
      (`PrimitiveComponent.SetMaterial` _staticmesh 1 "/Game/Materials/M_Top_Walked.M_Top_Walked")
      (set `self.TileType` "NewEnumerator0")
      (set `self.bCanWalk` true))
    (:`NewEnumerator1`
      (`PrimitiveComponent.SetMaterial` _staticmesh 1 "/Game/Materials/M_Top_CanWalk.M_Top_CanWalk")
      (set `self.TileType` "NewEnumerator1")
      (set `self.bCanWalk` true))
    (:`NewEnumerator2`
      (`PrimitiveComponent.SetMaterial` _staticmesh 1 "/Game/Materials/M_Top_CannotWalk.M_Top_CannotWalk")
      (set `self.TileType` "NewEnumerator2")
      (set `self.bCanWalk` false))
    (:`NewEnumerator3`
      (`PrimitiveComponent.SetMaterial` _staticmesh 1 "/Game/Materials/M_Top_Finish.M_Top_Finish")
      (set `self.TileType` "NewEnumerator3"))
    (:`NewEnumerator4`
      (`PrimitiveComponent.SetMaterial` _staticmesh 1 "/Game/Materials/M_Top_Black.M_Top_Black")
      (set `self.TileType` "NewEnumerator4")
      (set `self.bCanWalk` false))))

(fn `UserConstructionScript`)