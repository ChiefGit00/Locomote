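; BP_Tile is a clickable, touchable grid tile that sends BP_PlayerPawn to itself when walkable.
; Its type drives the top material and walkable state through SetTileType, also applied at construction.
; On BeginPlay it caches neighbouring tiles from CollX and CollY overlaps.
; OnWalked turns a Can Walk tile Walked and unlocks neighbouring Cannot Walk and Finish tiles; pawn overlap only prints debug walked or win messages.
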(event `self.ReceiveBeginPlay`
  (`self.GetNeighbours`))

(event `self.StaticMesh.OnClicked`
  (params (TouchedComponent :type "PrimitiveComponent Object Reference") (ButtonPressed :type "Key Structure"))
  (if (`self.bCanWalk`) :!label _label
    (bind _asbp_player_pawn (cast `/Game/Blueprints/Pawn/BP_PlayerPawn` (`GameplayStatics.GetPlayerPawn` 0)))
    (`/Game/Blueprints/Pawn/BP_PlayerPawn.MoveToTile` _asbp_player_pawn (+ (`self.K2_GetActorLocation`) (0.0 0.0 27.0)) self)))

(event `self.StaticMesh.OnInputTouchBegin`
  (params (FingerIndex :type "ETouchIndex Enum" :default "Touch1") (TouchedComponent :type "PrimitiveComponent Object Reference"))
  (goto _label))

(event `self.Box.OnComponentBeginOverlap`
  (params (OverlappedComponent :type "PrimitiveComponent Object Reference") (OtherActor :type "Actor Object Reference") (OtherComp :type "PrimitiveComponent Object Reference") (OtherBodyIndex :type Integer) (bFromSweep :type Boolean) (SweepResult :type "HitResult Structure (by ref)"))
  (cast `/Game/Blueprints/Pawn/BP_PlayerPawn` OtherActor)
  (switch `/Game/Data/E_TileType` (`self.TileType`)
    (:`NewEnumerator1`
      (`KismetSystemLibrary.PrintString` "Walked"))
    (:`NewEnumerator3`
      (`KismetSystemLibrary.PrintString` "Win"))))

(fn `ActivateNeighbour`
  (for _array_element (`self.NeighbourTiles`)
    (`/Engine/EditorBlueprintResources/StandardMacros.IsValid` _array_element
      (:`Is Valid`
        (bind _tiletype (`/Game/Blueprints/Actors/BP_Tile.TileType` _array_element))
        (if (`|EnumEquality` _tiletype "NewEnumerator2")
          (`self.SetTileType` _array_element "NewEnumerator1" false)
          (elif (`|EnumEquality` _tiletype "NewEnumerator3")
            (set `/Game/Blueprints/Actors/BP_Tile.bCanWalk` true _array_element)))))))

(fn `GetNeighbour`
  (params (Component :type "PrimitiveComponent Object Reference"))
  (returns (Tile :type "/Game/Blueprints/Actors/BP_Tile Object Reference"))
  (bind (_outactors _returnvalue) (`KismetSystemLibrary.ComponentOverlapActors` Component (`SceneComponent.K2_GetComponentToWorld` Component) (`|MakeArray` "ObjectTypeQuery2" :!type "EObjectTypeQuery Enum") "BP_Tile_C"))
  (if _returnvalue
    (for _array_element _outactors
      (bind _asbp_tile (cast `/Game/Blueprints/Actors/BP_Tile` _array_element))
      (break))
    (return _asbp_tile)))

(fn `GetNeighbours`
  (`KismetArrayLibrary.Array_Clear` (`self.NeighbourTiles`))
  (bind _tile (`self.GetNeighbour` (`self.Coll_X+`)))
  (`KismetArrayLibrary.Array_Add` (`self.NeighbourTiles`) _tile)
  (bind _tile_2 (`self.GetNeighbour` (`self.Coll_X-`)))
  (`KismetArrayLibrary.Array_Add` (`self.NeighbourTiles`) _tile_2)
  (bind _tile_3 (`self.GetNeighbour` (`self.Coll_Y+`)))
  (`KismetArrayLibrary.Array_Add` (`self.NeighbourTiles`) _tile_3)
  (bind _tile_4 (`self.GetNeighbour` (`self.Coll_Y-`)))
  (`KismetArrayLibrary.Array_Add` (`self.NeighbourTiles`) _tile_4))

(fn `OnWalked`
  (if (`|EnumEquality` (`self.TileType`) "NewEnumerator1")
    (`self.SetTileType` "NewEnumerator0" true)
    (`self.ActivateNeighbour`)))

(fn `SetTileType`
  (params (TileType :type "/Game/Data/E_TileType Enum" :default "NewEnumerator0") (bCanWalk :type Boolean))
  (bind _staticmesh (`self.StaticMesh`))
  (`|ExecutionSequence`
    (:`then_0`
      (switch `/Game/Data/E_TileType` TileType
        (:`NewEnumerator0`
          (`PrimitiveComponent.SetMaterial` _staticmesh 1 "/Game/Materials/MI_Top_Walked.MI_Top_Walked")
          (set `self.TileType` "NewEnumerator0")
          (set `self.bCanWalk` true))
        (:`NewEnumerator1`
          (`PrimitiveComponent.SetMaterial` _staticmesh 1 "/Game/Materials/MI_Top_CanWalkOn.MI_Top_CanWalkOn")
          (set `self.TileType` "NewEnumerator1")
          (set `self.bCanWalk` true))
        (:`NewEnumerator2`
          (`PrimitiveComponent.SetMaterial` _staticmesh 1 "/Game/Materials/MI_Top_CannotWalkOn.MI_Top_CannotWalkOn")
          (set `self.TileType` "NewEnumerator2"))
        (:`NewEnumerator3`
          (`PrimitiveComponent.SetMaterial` _staticmesh 1 "/Game/Materials/MI_Top_Finish.MI_Top_Finish")
          (set `self.TileType` "NewEnumerator3"))
        (:`NewEnumerator4`
          (`PrimitiveComponent.SetMaterial` _staticmesh 1 "/Game/Materials/MI_Top_Block.MI_Top_Block")
          (set `self.TileType` "NewEnumerator4")
          (set `self.bCanWalk` false))))))

(fn `UserConstructionScript`
  (`self.SetTileType` (`self.TileType`)))