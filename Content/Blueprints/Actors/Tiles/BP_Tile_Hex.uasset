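; Hexagonal tile actor, a child of a parent tile Blueprint that supplies the shared tile logic.
; Construction runs the parent script, then rebuilds the BoxColls array with six entries drawn from the CollX, CollXY and CollYX components, some repeated.
; BeginPlay calls GetNeighbours to find adjacent tiles.
; SetTileType only forwards to the parent implementation.
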(event `self.ReceiveBeginPlay`
  (`self.GetNeighbours`))

(fn `SetTileType`
  (params (TileType :type "/Game/Data/E_TileType Enum" :default "NewEnumerator0"))
  (`parent.SetTileType` TileType))

(fn `UserConstructionScript`
  (`parent.UserConstructionScript`)
  (`KismetArrayLibrary.Array_Clear` (`self.BoxColls`))
  (set `self.BoxColls` (`|MakeArray` (`self.Coll_X+`) (`self.Coll_X-`) (`self.Coll_X+Y+`) (`self.Coll_X-Y+`) (`self.Coll_X-Y-`) (`self.Coll_Y-X+`) :!type "PrimitiveComponent Object Reference")))