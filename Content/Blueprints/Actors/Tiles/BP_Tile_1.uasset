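; BP_Tile_1 is a tile actor that sets up its neighbour-detection colliders when play begins.
; On BeginPlay it rebuilds the BoxColls array from just two components, adding CollX twice and then CollY twice to give four entries.
; It then calls GetNeighbours, whose logic is not defined in this graph.
; The construction script only runs the parent's version.
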(event `self.ReceiveBeginPlay`
  (bind _boxcolls (`self.BoxColls`))
  (`KismetArrayLibrary.Array_Clear` _boxcolls)
  (`KismetArrayLibrary.Array_Add` _boxcolls (`self.Coll_X+`))
  (`KismetArrayLibrary.Array_Add` _boxcolls (`self.Coll_X-`))
  (`KismetArrayLibrary.Array_Add` _boxcolls (`self.Coll_Y+`))
  (`KismetArrayLibrary.Array_Add` _boxcolls (`self.Coll_Y-`))
  (`self.GetNeighbours`))

(fn `UserConstructionScript`
  (`parent.UserConstructionScript`))