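; BP_Tile_1D8_1C is a child tile Blueprint that adds a top-arrow indicator reflecting the tile's walk state.
; Its SetTileType override runs the parent logic, then casts the tile's widget to UI_TileTopArrow.
; The arrow shows, configured from IndexToActivate, only for Can Walk; Walked, Cannot Walk, Finish and Block hide it.
; BeginPlay and the construction script only call the parent.
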(event `self.ReceiveBeginPlay`
  (`parent.ReceiveBeginPlay`))

(fn `SetTileType`
  (params (TileType :type "/Game/Data/E_TileType Enum" :default "NewEnumerator0"))
  (`parent.SetTileType` TileType)
  (bind _asui_tile_top_arrow (cast `/Game/UI/UI_TileTopArrow` (`WidgetComponent.GetUserWidgetObject` (`self.Widget`))))
  (switch `/Game/Data/E_TileType` (`self.TileType`)
    (:`NewEnumerator0`
      (`/Game/UI/UI_TileTopArrow.Visible` _asui_tile_top_arrow false))
    (:`NewEnumerator1`
      (`/Game/UI/UI_TileTopArrow.Visible` _asui_tile_top_arrow true)
      (`/Game/UI/UI_TileTopArrow.Arrow` _asui_tile_top_arrow (`self.IndexToActivate`)))
    (:`NewEnumerator2`
      (`/Game/UI/UI_TileTopArrow.Visible` _asui_tile_top_arrow false :!label _label))
    (:`NewEnumerator3`
      (goto _label))
    (:`NewEnumerator4`
      (goto _label))))

(fn `UserConstructionScript`
  (`parent.UserConstructionScript`))