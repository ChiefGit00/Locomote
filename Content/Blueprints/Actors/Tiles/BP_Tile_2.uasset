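; Tile actor Blueprint, a child variant that looks up its neighbouring tiles when play begins.
; Its construction script runs the parent's, then rebuilds BoxColls as an eight-slot array from four directional colliders (X, Y, XY, YX), several of them repeated.
; BeginPlay calls GetNeighbours, which is not defined in this graph, and a leftover Delay node is never executed.
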(event `self.ReceiveBeginPlay`
  (`self.GetNeighbours`))

(fn `UserConstructionScript`
  (`parent.UserConstructionScript`)
  (`KismetArrayLibrary.Array_Clear` (`self.BoxColls`))
  (set `self.BoxColls` (`|MakeArray` (`self.Coll_X+`) (`self.Coll_X-`) (`self.Coll_Y+`) (`self.Coll_Y-`) (`self.Coll_X+Y+`) (`self.Coll_X-Y+`) (`self.Coll_X-Y-`) (`self.Coll_Y-X+`) :!type "PrimitiveComponent Object Reference")))