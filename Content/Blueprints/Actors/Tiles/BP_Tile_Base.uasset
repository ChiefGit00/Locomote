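; Base tile actor for a tile-walking level, where clicking or touching a walkable tile tells the player controller to move there.
; A tile type drives the top material and walkability.
; Box-collision overlaps find neighbours, which walked tiles unlock (all or one chosen index) and DeactivateUnused locks again.
; Finish tiles toggle between active and inactive looks and fetch the XP award from the parent BP_Level.
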(event `self.StaticMesh.OnClicked`
  (params (TouchedComponent :type "PrimitiveComponent Object Reference") (ButtonPressed :type "Key Structure"))
  (`self.OnClicked/Touched` :!label _label))

(event `self.StaticMesh.OnInputTouchBegin`
  (params (FingerIndex :type "ETouchIndex Enum" :default "Touch1") (TouchedComponent :type "PrimitiveComponent Object Reference"))
  (goto _label))

(fn `ActivateNeighbours`
  (bind _output (`|GetArrayItem` (`self.NeighbourTiles`) (`self.IndexToActivate`)))
  (bind _tiletype (`/Game/Blueprints/Actors/Tiles/BP_Tile_Base.TileType` _output))
  (if (not (`self.bActivateOne`))
    (for _array_element (`self.NeighbourTiles`)
      (`/Engine/EditorBlueprintResources/StandardMacros.IsValid` _array_element
        (:`Is Valid`
          (bind _tiletype_2 (`/Game/Blueprints/Actors/Tiles/BP_Tile_Base.TileType` _array_element))
          (if (`|EnumEquality` _tiletype_2 "NewEnumerator2")
            (`self.SetTileType` _array_element "NewEnumerator1")
            (elif (`|EnumEquality` _tiletype_2 "NewEnumerator3")
              (set `/Game/Blueprints/Actors/Tiles/BP_Tile_Base.bCanWalk` true _array_element)
              (`self.SetTileType` _array_element "NewEnumerator3"))))))
    (else
      (`/Engine/EditorBlueprintResources/StandardMacros.IsValid` _output
        (:`Is Valid`
          (if (`|EnumEquality` _tiletype "NewEnumerator2")
            (`self.SetTileType` _output "NewEnumerator1")
            (elif (`|EnumEquality` _tiletype "NewEnumerator3")
              (set `/Game/Blueprints/Actors/Tiles/BP_Tile_Base.bCanWalk` true _output)
              (`self.SetTileType` _output "NewEnumerator3"))))))))

(fn `DeactivateUnused`
  (params (A :type Integer) (Index :type Boolean))
  (set `self.bCanWalk` true)
  (for _array_element (`self.NeighbourTiles`)
    (`/Engine/EditorBlueprintResources/StandardMacros.IsValid` _array_element
      (:`Is Valid`
        (bind _tiletype (`/Game/Blueprints/Actors/Tiles/BP_Tile_Base.TileType` _array_element))
        (if (`|EnumEquality` _tiletype "NewEnumerator1")
          (`self.SetTileType` _array_element "NewEnumerator2")
          (elif (`|EnumEquality` _tiletype "NewEnumerator3")
            (set `/Game/Blueprints/Actors/Tiles/BP_Tile_Base.bCanWalk` false _array_element)
            (`self.SetTileType` _array_element "NewEnumerator3")))))))

(fn `GetNeighbour`
  (params (BoxCollision :type "PrimitiveComponent Object Reference"))
  (returns (Tile :type "/Game/Blueprints/Actors/Tiles/BP_Tile_Base Object Reference"))
  (bind (_outactors _returnvalue) (`KismetSystemLibrary.ComponentOverlapActors` BoxCollision (`SceneComponent.K2_GetComponentToWorld` BoxCollision) (`|MakeArray` "ObjectTypeQuery2" :!type "EObjectTypeQuery Enum") "BP_Tile_Base_C" (`|MakeArray` self :!type "Actor Object Reference")))
  (if _returnvalue
    (bind _asbp_tile_base (cast `/Game/Blueprints/Actors/Tiles/BP_Tile_Base` (`|GetArrayItem` _outactors)))
    (return _asbp_tile_base)
    (else
      (return null))))

(fn `GetNeighbours`
  (`KismetArrayLibrary.Array_Clear` (`self.NeighbourTiles`))
  (for _array_element (`self.BoxColls`)
    (bind _tile (`self.GetNeighbour` _array_element))
    (`/Engine/EditorBlueprintResources/StandardMacros.IsValid` _tile
      (:`Is Valid`
        (`KismetArrayLibrary.Array_Add` (`self.NeighbourTiles`) _tile)))))

(fn `GetXPAward`
  (returns (XP :type Integer))
  (set `self.bCanWalk` true)
  (`self.SetTileType` "NewEnumerator3")
  (bind _asbp_level (cast `/Game/Blueprints/Actors/Levles/BP_Level` (`self.GetParentActor`)))
  (return (`/Game/Blueprints/Actors/Levles/BP_Level.XPAward` _asbp_level)))

(fn `OnClicked/Touched`
  (if (`self.bCanWalk`)
    (bind _asbp_player_ctrl_levels (cast `/Game/Blueprints/Game/BP_PlayerCtrl_Levels` (`GameplayStatics.GetPlayerController` 0)))
    (`/Game/Blueprints/Game/BP_PlayerCtrl_Levels.Move` _asbp_player_ctrl_levels (+ (`self.K2_GetActorLocation`) (0.0 0.0 27.0)) self)))

(fn `OnWalked`
  (if (`|EnumInequality` (`self.TileType`) "NewEnumerator3")
    (`self.SetTileType` "NewEnumerator0")
    (set `self.bCanWalk` false)
    (`self.ActivateNeighbours`)
    (else
      (set `self.bCanWalk` true))))

(fn `SetTileType`
  (params (TileType :type "/Game/Data/E_TileType Enum" :default "NewEnumerator0"))
  (bind _staticmesh (`self.StaticMesh`))
  (switch `/Game/Data/E_TileType` TileType
    (:`NewEnumerator0`
      (`PrimitiveComponent.SetMaterial` _staticmesh 1 "/Game/Materials/M_Top_Walked.M_Top_Walked")
      (set `self.TileType` "NewEnumerator0")
      (set `self.bCanWalk` true))
    (:`NewEnumerator1`
      (`PrimitiveComponent.SetMaterial` _staticmesh 1 "/Game/Materials/M_Top_CanWalk.M_Top_CanWalk")
      (set `self.TileType` "NewEnumerator1")
      (set `self.bCanWalk` true))
    (:`NewEnumerator2`
      (`PrimitiveComponent.SetMaterial` _staticmesh 1 "/Game/Materials/M_Top_CannotWalk.M_Top_CannotWalk")
      (set `self.TileType` "NewEnumerator2")
      (set `self.bCanWalk` false))
    (:`NewEnumerator3`
      (if (`self.bCanWalk`)
        (`PrimitiveComponent.SetMaterial` _staticmesh 1 "/Game/Materials/M_Top_Finish_active.M_Top_Finish_active")
        (else
          (`PrimitiveComponent.SetMaterial` _staticmesh 1 "/Game/Materials/M_Top_Finish_deactive.M_Top_Finish_deactive")))
      (set `self.TileType` "NewEnumerator3"))
    (:`NewEnumerator4`
      (`PrimitiveComponent.SetMaterial` _staticmesh 1 "/Game/Materials/M_Top_Black.M_Top_Black")
      (set `self.TileType` "NewEnumerator4")
      (set `self.bCanWalk` false))))

(fn `UserConstructionScript`
  (`self.SetTileType` (`self.TileType`)))