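; Hex tile variant that continuously cycles down and up, and is clickable only during a pause after rising.
; BeginPlay gathers neighbours, then chains GoDown and ComeUp timelines that add Z offsets to the static mesh each update.
; After rising it briefly enables CanClick and swaps the Box material, then reverts both and restarts the descent.
; Construction refills the BoxColls collision list after the parent script; SetTileType defers to the parent.
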(event `self.ReceiveBeginPlay`
  (`self.GetNeighbours`)
  (`self.Move`))

(event `Move`
  (bind (_direction _newtrack_0) (`Timeline|GoDown` :!label _label)
    (:`Update`
      (`SceneComponent.K2_AddRelativeLocation` (`self.StaticMesh`) (`KismetMathLibrary.MakeVector` 0.0 0.0 _newtrack_0) false false))
    (:`Finished`
      (bind (_direction_2 _z) (`Timeline|ComeUp` :!via `PlayFromStart`)
        (:`Update`
          (`SceneComponent.K2_AddRelativeLocation` (`self.StaticMesh`) (`KismetMathLibrary.MakeVector` 0.0 0.0 _z) false false))
        (:`Finished`
          (set `self.bCanClick` true)
          (`PrimitiveComponent.SetMaterial` (`self.Box`) 0 "/Game/Materials/M_Bottom.M_Bottom")
          (`KismetSystemLibrary.Delay` 2.0)
          (set `self.bCanClick` false)
          (`PrimitiveComponent.SetMaterial` (`self.Box`) 0 "/Engine/EngineMaterials/WorldGridMaterial_Low.WorldGridMaterial_Low")
          (goto _label :!via `PlayFromStart`))))))

(fn `SetTileType`
  (params (TileType :type "/Game/Data/E_TileType Enum" :default "NewEnumerator0"))
  (`parent.SetTileType` TileType))

(fn `UserConstructionScript`
  (`parent.UserConstructionScript`)
  (`KismetArrayLibrary.Array_Clear` (`self.BoxColls`))
  (set `self.BoxColls` (`|MakeArray` (`self.Coll_X+`) (`self.Coll_X-`) (`self.Coll_X+Y+`) (`self.Coll_X-Y+`) (`self.Coll_X-Y-`) (`self.Coll_Y-X+`) :!type "PrimitiveComponent Object Reference")))